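; Procedural generation actor that builds a jagged line by midpoint displacement from a hardcoded segment on BeginPlay.
; Each iteration replaces every segment with two, offsetting the midpoint by a constant DisplacementAmount along a normalized vector perpendicular in XY, with no randomness or falloff.
; Tick draws the resulting Lines and the two original endpoints stored in Points.
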(event EventBeginPlay
  (bind _fs_point (Utilities|Struct|MakeFS_Point "0.000000,0.000000,10.000000" "(R=1.000000,G=0.000000,B=0.000000,A=1.000000)"))
  (bind _fs_point_2 (Utilities|Struct|MakeFS_Point "500.000000,0.000000,10.000000" "(R=1.000000,G=0.000000,B=0.000000,A=1.000000)"))
  (Utilities|Array|AddUnique (Variables|Default|GetPoints) _fs_point)
  (Utilities|Array|AddUnique (Variables|Default|GetPoints) _fs_point_2)
  (Midpoint-Displacement|MidpointDisplacement _fs_point _fs_point_2))

(event Collision|EventActorBeginOverlap
  (params (OtherActor :type Actor%20Object%20Reference)))

(event EventTick
  (params (DeltaSeconds :type Float%20%28single-precision%29))
  (CallFunction|DrawPoints (Variables|Default|GetPoints))
  (CallFunction|DrawLines (Variables|Default|GetLines)))

(fn ConstructionScript)

(fn MidpointDisplacement
  (params (FirstStartPoint :type FS%20Point%20Structure) (FirstEndPoint :type FS%20Point%20Structure))
  (bind _lines (Variables|Default|GetLines))
  (bind _segments (LocalVariables|GetSegments))
  (Utilities|Array|AddUnique (LocalVariables|GetSegments) (Utilities|Struct|MakeFS_Line FirstStartPoint FirstEndPoint))
  (for _index (range 0 (- (Variables|Midpoint-Displacement|GetIteration) 1))
    (LocalVariables|SetTempSegments _segments)
    (Utilities|Array|Clear _segments)
    (for _array_element (LocalVariables|GetTempSegments)
      (bind _segments_2 (Midpoint-Displacement|DisplaceMidPoint _array_element))
      (Utilities|Array|AppendArray (LocalVariables|GetSegments) _segments_2)))
  (Utilities|Array|Clear _lines)
  (Utilities|Array|AppendArray _lines (LocalVariables|GetSegments)))

(fn FindMiddlePoint
  (params (Line :type FS%20Line%20Structure))
  (bind (_startpoint _endpoint) (Utilities|Struct|BreakFS_Line Line))
  (bind _pointlocation (Utilities|Struct|BreakFS_Point _startpoint))
  (bind (_pointlocation_2 _color _type) (Utilities|Struct|BreakFS_Point _endpoint))
  (return (Utilities|Struct|MakeFS_Point (+ _pointlocation (/ (- _pointlocation_2 _pointlocation) 2)) _color _type)))

(fn DisplaceMidPoint
  (params (Line :type FS%20Line%20Structure))
  (bind (_startpoint _endpoint) (Utilities|Struct|BreakFS_Line Line))
  (LocalVariables|SetTempStart _startpoint)
  (LocalVariables|SetTempEnd _endpoint)
  (bind _middlepoint (Midpoint-Displacement|FindMiddlePoint Line))
  (return (Utilities|Array|MakeArray (Utilities|Struct|MakeFS_Line (LocalVariables|GetTempStart) (Utilities|Struct|MakeFS_Point (+ (.pointlocation _middlepoint) (* (Math|Vector|Normalize (Math|Vector|MakeVector (.Y (Math|Vector|BreakVector (- (.pointlocation (LocalVariables|GetTempEnd)) (.pointlocation (LocalVariables|GetTempStart))))) (* (.X (Math|Vector|BreakVector (- (.pointlocation (LocalVariables|GetTempEnd)) (.pointlocation (LocalVariables|GetTempStart))))) -1.0) (.Z (Math|Vector|BreakVector (- (.pointlocation (LocalVariables|GetTempEnd)) (.pointlocation (LocalVariables|GetTempStart))))))) (Variables|Midpoint-Displacement|GetDisplacementAmount))) (.color _middlepoint) (.type _middlepoint))) (Utilities|Struct|MakeFS_Line (Utilities|Struct|MakeFS_Point (+ (.pointlocation _middlepoint) (* (Math|Vector|Normalize (Math|Vector|MakeVector (.Y (Math|Vector|BreakVector (- (.pointlocation (LocalVariables|GetTempEnd)) (.pointlocation (LocalVariables|GetTempStart))))) (* (.X (Math|Vector|BreakVector (- (.pointlocation (LocalVariables|GetTempEnd)) (.pointlocation (LocalVariables|GetTempStart))))) -1.0) (.Z (Math|Vector|BreakVector (- (.pointlocation (LocalVariables|GetTempEnd)) (.pointlocation (LocalVariables|GetTempStart))))))) (Variables|Midpoint-Displacement|GetDisplacementAmount))) (.color _middlepoint) (.type _middlepoint)) (LocalVariables|GetTempEnd)))))